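; Base inspectable item that the player can bring up to the camera and rotate, with its name and description shown on screen.
; BeginInteract and EndInteract toggle its widget, while Interact disables collision, attaches it to the camera manager, glides it forward and hands input from player to item.
; Holding left mouse rotates it through yaw and pitch.
; IA_Interact detaches it, removes the UI, returns it to its BeginPlay transform and restores player input.
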(event `/Game/Item_Inspect_System/Blueprint/BP_Inspect_Interface.BeginInteract`
  ;[1 1 1] Set Widget Visibility
  (`SceneComponent.SetVisibility` (`self.Widget`) true false))

(event `/Game/Item_Inspect_System/Blueprint/BP_Inspect_Interface.EndInteract`
  ;[1 1 1] Set Widget Visibility
  (`SceneComponent.SetVisibility` (`self.Widget`) false false))

(event `self.ReceiveBeginPlay`
  ;[0 0 0] Comment
  ;;[1 1 1] Begin Play
  (set `self.Transform` (`self.GetTransform`)))

(event `/Game/Item_Inspect_System/Blueprint/BP_Inspect_Interface.Interact`
  (params (Player :type "Character Object Reference"))
  (bind _returnvalue (`GameplayStatics.GetPlayerController` 0))
  ;[0 0 0] Comment
  ;;[1 1 1] Attach
  (if (not (`self.Condition`))
    (set `self.Condition` true)
    (set `self.Player_Ref` Player)
    (`self.SetActorEnableCollision` false)
    (`self.K2_AttachToComponent` (`PlayerCameraManager.TransformComponent` (`GameplayStatics.GetPlayerCameraManager` 0)) "None" "KeepWorld" "KeepWorld" "KeepWorld")
    (bind _returnvalue_2 (`|CreateWidget` "/Game/Item_Inspect_System/Widget/UI_Intespect.UI_Intespect_C" null (`self.ItemName`) (`self.ItemDescription`) (`self.State`)))
    (bind _output_get (set `self.InspectUI` _returnvalue_2))
    (`UserWidget.AddToViewport` _output_get 0)
    ;;;[1 1 1] item widget removal = Target Relative Location
    (`KismetSystemLibrary.MoveComponentTo` (`self.DefaultSceneRoot`) (200.0 0.0 0.0))
    ;;;[1 1 1] Player Input
    (`self.DisableInput` (`self.Player_Ref`) _returnvalue)
    (`self.EnableInput` _returnvalue)
    ;;;[1 1 1] Interact Delay
    (`KismetSystemLibrary.Delay` 2.0)
    (set `self.Condition` false)))

(event `EnhancedInput|/Game/Input/Actions/IA_Interact`
  (params (ActionValue :type Boolean) (ElapsedSeconds :type "Float (double-precision)") (TriggeredSeconds :type "Float (double-precision)") (InputAction :type "InputAction Object Reference" :default "/Game/Input/Actions/IA_Interact.IA_Interact"))
  (bind _returnvalue (`GameplayStatics.GetPlayerController` 0))
  (bind (_transform_location _transform_rotation) (`KismetMathLibrary.BreakTransform` (`self.Transform`)))
  ;[0 0 0] Comment
  (:`Triggered`
    ;;[1 1 1] Detach
    (`self.K2_DetachFromActor` "KeepWorld" "KeepWorld" "KeepWorld")
    (`Widget.RemoveFromParent` (`self.InspectUI`))
    (set `self.InspectUI` null)
    (`KismetSystemLibrary.MoveComponentTo` (`self.DefaultSceneRoot`) _transform_location _transform_rotation)
    (`self.SetActorEnableCollision` true)
    (`self.DisableInput` _returnvalue)
    (`self.EnableInput` (`self.Player_Ref`) _returnvalue)))

(event `Key|LeftMouseButton`
  (params (Key :type "Key Structure"))
  ;[0 0 0] Comment
  ;;[1 1 1] Item Rotation Controls
  (:`Pressed`
    (set `self.CanRotate` true))
  (:`Released`
    (set `self.CanRotate` false)))

(event `InputAxisKey|MouseX`
  (params (AxisValue :type "Float (single-precision)"))
  ;[0 0 0] Comment
  ;;[1 1 1] Item Rotation Controls
  (if (`self.CanRotate`)
    (`self.K2_SetActorRotation` (`KismetMathLibrary.ComposeRotators` (`self.K2_GetActorRotation`) (`KismetMathLibrary.MakeRotator` 0.0 0.0 (* AxisValue -2.0))))))

(event `InputAxisKey|MouseY`
  (params (AxisValue :type "Float (single-precision)"))
  ;[0 0 0] Comment
  ;;[1 1 1] Item Rotation Controls
  (if (`self.CanRotate`)
    (`self.K2_SetActorRotation` (`KismetMathLibrary.ComposeRotators` (`self.K2_GetActorRotation`) (`KismetMathLibrary.MakeRotator` 0.0 (* AxisValue 2.0))))))

(fn `CanTrace`
  (params (CanInteract :type Boolean))
  (return))

(fn `UserConstructionScript`)